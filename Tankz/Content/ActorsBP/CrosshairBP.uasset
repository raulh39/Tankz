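; Crosshair actor that spins continuously and shows whether it is selected through its emissive color.
; The construction script creates a dynamic material instance on the Crosshair component, and Tick rolls that component at a constant, frame-rate-independent speed.
; The SetSelected event calls SetSelectedImpl, which sets the Emissive parameter to teal when selected and to the unassigned NewParameter value otherwise.
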(event `self.ReceiveTick`
  (params (DeltaSeconds :type "Float (single-precision)"))
  (`SceneComponent.K2_AddLocalRotation` (`self.Crosshair`) (`KismetMathLibrary.MakeRotator` (* DeltaSeconds 100.0)) false false))

(event `self.SetSelected`
  (params (isSelected :type Boolean))
  (`self.SetSelectedImpl` isSelected))

(fn `SetSelectedImpl`
  (params (IsSelected :type Boolean))
  (locals (NewParameter :type "LinearColor Structure"))
  (if IsSelected
    (set `local.NewParameter` (make `LinearColor` 0.0 0.6 0.6)))
  (`MaterialInstanceDynamic.SetVectorParameterValue` (`self.CrossMaterial`) "Emissive" (`local.NewParameter`)))

(fn `UserConstructionScript`
  (bind _returnvalue (`PrimitiveComponent.CreateDynamicMaterialInstance` (`self.Crosshair`) 0 "/Game/Materials/CrosshairMaterialInstance.CrosshairMaterialInstance"))
  (set `self.CrossMaterial` _returnvalue))