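; Base tank actor Blueprint that controls the hull's appearance for selection highlighting and base color.
; The construction script creates a dynamic material instance on the Hull and stores it as HullMaterial.
; SetSelected and SetBaseColor events forward to implementation functions that write that material's vector parameters.
; Selection sets an overbright red emissive color, while deselection applies the unassigned default color.
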(event `self.SetSelected`
  (params (isSelected :type Boolean))
  (`self.SetSelectedImpl` isSelected))

(event `self.SetBaseColor`
  (params (newBaseColor :type "LinearColor Structure"))
  (`self.SetBaseColorImpl` newBaseColor))

(fn `SetBaseColorImpl`
  (params (NewBaseColor :type "LinearColor Structure"))
  (`MaterialInstanceDynamic.SetVectorParameterValue` (`self.HullMaterial`) "BaseColor" NewBaseColor))

(fn `SetSelectedImpl`
  (params (isSelected :type Boolean))
  (locals (NewColor :type "LinearColor Structure"))
  (if isSelected
    (set `local.NewColor` (make `LinearColor` 5.0 0.5 0.5)))
  (`MaterialInstanceDynamic.SetVectorParameterValue` (`self.HullMaterial`) "EmissiveColor" (`local.NewColor`)))

(fn `UserConstructionScript`
  (bind _returnvalue (`PrimitiveComponent.CreateDynamicMaterialInstance` (`self.Hull`) 0 "/Game/Materials/TankMaterialInstance.TankMaterialInstance"))
  (set `self.HullMaterial` _returnvalue))